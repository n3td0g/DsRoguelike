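; BP_DungeonGenerator starts dungeon generation and places the player's character in the result for a roguelike game.
; It calls GenerateDungeon on BeginPlay; the generation logic itself is not in these graphs.
; When the DungeonGenerated event fires, it takes the center of the first room, if any exist, and passes it to BP_PlayerController's SpawnCharacter.
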(event EventBeginPlay
  (Class|DungeonGenerator|GenerateDungeon))

(event EventDungeonGenerated
  (bind _rooms (Variables|Default|GetRooms))
  (if (> (Utilities|Array|Length _rooms) 0)
    (bind _returnvalue (Class|DungeonGenerator|GetRoomCenter (Utilities|Array|Get(acopy) _rooms)))
    (bind _asbp_player_controller (Utilities|Casting|CastToBP_PlayerController (Game|GetPlayerController 0)))
    (Default|SpawnCharacter _asbp_player_controller _returnvalue)))

(fn ConstructionScript)