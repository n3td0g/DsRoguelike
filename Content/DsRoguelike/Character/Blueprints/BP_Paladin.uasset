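; Paladin character Blueprint for a roguelike that adds a roll on the Space Bar.
; StartRolling ignores repeat presses while rolling, shrinks the capsule's half height and stores the current yaw as RollDirection.
; StopRolling clears the flag, restores the capsule and rotates the actor back to the stored yaw.
; Nothing in this Blueprint calls StopRolling or moves the character during the roll.
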(event EventBeginPlay)

(event Input|KeyboardEvents|SpaceBar
  (params (Key :type Key%20Structure))
  (:Pressed
    (CallFunction|StartRolling)))

(fn ConstructionScript)

(fn StartRolling
  (if (not (Variables|Default|GetIsRolling))
    (Variables|Default|SetIsRolling true)
    (Components|Capsule|SetCapsuleHalfHeight (Variables|Default|GetCapsuleComponent) 42.0 false)
    (Variables|Default|SetRollDirection (.yaw (Transformation|GetActorRotation)))))

(fn StopRolling
  (Variables|Default|SetIsRolling false)
  (Components|Capsule|SetCapsuleHalfHeight (Variables|Default|GetCapsuleComponent) 96.0 false)
  (Transformation|SetActorRotation (Math|Rotator|MakeRotator 0.0 0.0 (Variables|Default|GetRollDirection))))